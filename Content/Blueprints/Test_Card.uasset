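; Test card Blueprint that plays a lift-and-flip animation when play begins.
; BeginPlay caches the card picture's relative location, a raised point above it and a half-turn pitch rotation.
; A timeline's separate Move and Angle tracks drive location and rotation lerps into a relative transform update each tick.
; An actor-level version of the same transform update is left unconnected.
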(event `self.ReceiveBeginPlay`
  (bind _output_get (set `self.StartLocation` (`SceneComponent.RelativeLocation` (`self.Card_Picture`))))
  (set `self.TempLocation` (+ _output_get (0.0 0.0 50.0)))
  (set `self.StartRotation` (struct))
  (set `self.EndRotation` (`KismetMathLibrary.MakeRot` 180.0))
  (bind (_direction _angle _move) (`Timeline|Timeline_0`)
    (:`Update`
      (`SceneComponent.K2_SetRelativeTransform` (`KismetMathLibrary.MakeTransform` (`KismetMathLibrary.VLerp` (`self.StartLocation`) (`self.TempLocation`) _move) (`KismetMathLibrary.RLerp` (`self.StartRotation`) (`self.EndRotation`) _angle))))))

(fn `UserConstructionScript`)